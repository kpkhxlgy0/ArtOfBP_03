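; BP_Camera is an actor that slowly turns its Camera1 component to follow the first player character.
; Each Tick interpolates the camera's forward vector toward the unnormalized vector to the player, then converts it to a rotation with zero roll.
; Pitch and yaw pass through angle clamps centered on the newly computed angles themselves, so the clamps never restrict the rotation.
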(event `self.ReceiveTick`
  (params (DeltaSeconds :type "Float (single-precision)"))
  (bind _pitch (.pitch (`KismetMathLibrary.MakeRotFromX` (`KismetMathLibrary.VInterpTo` (`KismetMathLibrary.Conv_RotatorToVector` (`SceneComponent.K2_GetComponentRotation` (`self.Camera1`))) (- (`self.K2_GetActorLocation` (`GameplayStatics.GetPlayerCharacter` 0)) (`SceneComponent.K2_GetComponentLocation` (`self.Camera1`))) (`self.DT_DeltaTime`) 0.01))))
  (bind _yaw (.yaw (`KismetMathLibrary.MakeRotFromX` (`KismetMathLibrary.VInterpTo` (`KismetMathLibrary.Conv_RotatorToVector` (`SceneComponent.K2_GetComponentRotation` (`self.Camera1`))) (- (`self.K2_GetActorLocation` (`GameplayStatics.GetPlayerCharacter` 0)) (`SceneComponent.K2_GetComponentLocation` (`self.Camera1`))) (`self.DT_DeltaTime`) 0.01))))
  (set `self.DT_DeltaTime` DeltaSeconds)
  (`SceneComponent.K2_SetWorldRotation` (`self.Camera1`) (`KismetMathLibrary.MakeRotator` 0.0 (`KismetMathLibrary.ClampAngle` _pitch (- _pitch 80.0) (+ _pitch 80.0)) (`KismetMathLibrary.ClampAngle` _yaw (- _yaw 80.0) (+ _yaw 80.0))) true false))

(fn `UserConstructionScript`)