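; BP_Pickup is a collectible item that comes in two types, a tin or a button, selected by PickupType.
; The construction script sets the pickup mesh to match the type.
; When the player character overlaps its box, it calls the matching PickedUpTin or PickedUpButton function on ThirdPersonCharacter, then destroys itself.
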(event `self.Box1.OnComponentBeginOverlap`
  (params (OverlappedComponent :type "PrimitiveComponent Object Reference") (OtherActor :type "Actor Object Reference") (OtherComp :type "PrimitiveComponent Object Reference") (OtherBodyIndex :type Integer) (bFromSweep :type Boolean) (SweepResult :type "HitResult Structure (by ref)"))
  (if (== OtherActor (`GameplayStatics.GetPlayerCharacter` 0))
    (switch `int` (`self.PickupType`)
      (:`0`
        (bind _asthird_person_character (cast `/Game/ThirdPersonBP/Blueprints/ThirdPersonCharacter` (`GameplayStatics.GetPlayerCharacter` 0)))
        (`/Game/ThirdPersonBP/Blueprints/ThirdPersonCharacter.PickedUpTin` _asthird_person_character))
      (:`1`
        (bind _asthird_person_character_2 (cast `/Game/ThirdPersonBP/Blueprints/ThirdPersonCharacter` (`GameplayStatics.GetPlayerCharacter` 0)))
        (`/Game/ThirdPersonBP/Blueprints/ThirdPersonCharacter.PickedUpButton` _asthird_person_character_2)))
    (`self.K2_DestroyActor`)))

(fn `UserConstructionScript`
  (switch `int` (`self.PickupType`)
    (:`0`
      (`StaticMeshComponent.SetStaticMesh` (`self.PickUpMesh`) "/Game/ArtOfBP/SM_Tin.SM_Tin"))
    (:`1`
      (`StaticMeshComponent.SetStaticMesh` (`self.PickUpMesh`) "/Game/ArtOfBP/SM_Button.SM_Button"))))